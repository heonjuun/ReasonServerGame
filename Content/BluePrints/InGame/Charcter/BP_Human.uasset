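; BP_Human is a human character with server-authoritative melee attacks, damage and ragdoll death.
; Attack-hit events sphere-trace forward and damage other humans, while attack-end returns the state to IdleMove.
; Incoming damage lowers HP toward a rock death, yet also immediately triggers normal death in Idle Move or Attack, notifying BP_GameMode when a BP_Player caused it.
; Both death events disable movement and capsule collision, then enable mesh physics.
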(event `self.ReceiveAnyDamage`
  (params (Damage :type "Float (single-precision)") (DamageType :type "DamageType Object Reference") (InstigatedBy :type "Controller Object Reference") (DamageCauser :type "Actor Object Reference"))
  (`/Engine/EditorBlueprintResources/ActorMacros.Switch Has Authority`
    (:`Authority`
      (`self.ApplyRockDamage` Damage)
      (switch `/Game/BluePrints/Enum/E_State` (`self.State`)
        (:`NewEnumerator0`
          _)
        (:`NewEnumerator1`
          _))
      (`|ExecutionSequence`
        (:`then_0`
          (`self.S2M_Death`))
        (:`then_1`
          (bind _asbp_game_mode (cast `/Game/BluePrints/InGame/BP_GameMode` (`GameplayStatics.GetGameMode`)))
          (bind _asbp_player (cast `/Game/BluePrints/InGame/Charcter/Player/BP_Player` DamageCauser))
          (`/Game/BluePrints/InGame/BP_GameMode.OnHumanDeath` _asbp_game_mode _asbp_player self))))))

(event `S2M_Death`
  (bind _mesh (`self.Mesh`))
  (`|ExecutionSequence`
    (:`then_0`
      (set `self.State` "NewEnumerator2"))
    (:`then_1`
      (`CharacterMovementComponent.DisableMovement` (`self.CharacterMovement`)))
    (:`then_2`
      (`PrimitiveComponent.SetCollisionEnabled` (`self.CapsuleComponent`) "NoCollision"))
    (:`then_3`
      (`PrimitiveComponent.SetCollisionEnabled` _mesh "PhysicsOnly")
      (`PrimitiveComponent.SetSimulatePhysics` _mesh true))))

(event `S2M_RockDeath`
  (bind _mesh (`self.Mesh`))
  (`PrimitiveComponent.SetCollisionResponseToChannel` (`self.Mesh`) "ECC_Pawn" "ECR_Ignore")
  (`CharacterMovementComponent.DisableMovement` (`self.CharacterMovement`))
  (`PrimitiveComponent.SetCollisionEnabled` (`self.CapsuleComponent`) "NoCollision")
  (`PrimitiveComponent.SetCollisionEnabled` _mesh "PhysicsOnly")
  (`PrimitiveComponent.SetSimulatePhysics` _mesh true))

(event `CallAttackEnd`
  (switch `/Game/BluePrints/Enum/E_State` (`self.State`)
    (:`NewEnumerator1`
      (set `self.State` "NewEnumerator0"))))

(event `CallAttackHit`
  (bind _returnvalue (`self.K2_GetActorLocation`))
  (`/Engine/EditorBlueprintResources/ActorMacros.Switch Has Authority`
    (:`Authority`
      (bind _outhits (`KismetSystemLibrary.SphereTraceMultiForObjects` :`Start` _returnvalue :`End` (+ _returnvalue (* (`self.GetActorForwardVector`) (`self.AttackRange`))) :`Radius` 15.0 :`ObjectTypes` (`|MakeArray` "ObjectTypeQuery3" :!type "EObjectTypeQuery Enum") :`DrawDebugType` "ForDuration"))
      (for _array_element _outhits
        (bind _asbp_human (cast `/Game/BluePrints/InGame/Charcter/BP_Human` (`.HitActor` (`GameplayStatics.BreakHitResult` _array_element))))
        (`GameplayStatics.ApplyDamage` _asbp_human 50.0 null self)))))

(fn `ApplyRockDamage`
  (params (DamageAmount :type "Float (double-precision)"))
  (if (not (`self.bIsDead`))
    (set `self.CurrentHp` (`KismetMathLibrary.FClamp` (- (`self.CurrentHp`) DamageAmount) 0.0 (`self.MaxHp`)))
    (if (<= (`self.CurrentHp`) 0.0)
      (`self.Die`))))

(fn `Die`
  (`/Engine/EditorBlueprintResources/ActorMacros.Switch Has Authority`
    (:`Authority`
      (if (not (`self.bIsDead`))
        (set `self.bIsDead` true)
        (set `self.CurrentHp` 0.0)
        (`self.S2M_RockDeath`)))))

(fn `UserConstructionScript`)