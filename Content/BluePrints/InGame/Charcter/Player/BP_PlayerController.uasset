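; BP_PlayerController is the player controller that turns Enhanced Input actions into control of the possessed BP_Player.
; On BeginPlay it caches the controlled pawn as BP_Player and, if that cast succeeds, adds the IMC_Default mapping context.
; Look drives controller yaw and pitch, while movement follows the control rotation with pitch zeroed.
; Jump and crouch start and stop with their inputs, and attack calls CallAttackInput on both Started and Triggered.
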(event `self.ReceiveBeginPlay`
  (bind _returnvalue (pcsubsystem `EnhancedInputLocalPlayerSubsystem` self))
  (bind _asbp_player (cast `/Game/BluePrints/InGame/Charcter/Player/BP_Player` (`self.K2_GetPawn`)))
  (set `self.AsBpPlayer` _asbp_player)
  (`/Engine/EditorBlueprintResources/StandardMacros.IsValid` _returnvalue
    (:`Is Valid`
      (`EnhancedInputSubsystemInterface.AddMappingContext` _returnvalue "/Game/BluePrints/Input/IMC_Default.IMC_Default" 0 (struct)))))

(event `EnhancedInput|/Game/BluePrints/Input/Action/IA_Look`
  (params (ActionValue :type "Vector2D Structure") (ElapsedSeconds :type "Float (double-precision)") (TriggeredSeconds :type "Float (double-precision)") (InputAction :type "InputAction Object Reference" :default "/Game/BluePrints/Input/Action/IA_Look.IA_Look"))
  (bind (_x _y) (`KismetMathLibrary.BreakVector2D` ActionValue))
  (:`Triggered`
    (`self.AddYawInput` _x)
    (`self.AddPitchInput` _y)))

(event `EnhancedInput|/Game/BluePrints/Input/Action/IA_Jump`
  (params (ActionValue :type Boolean) (ElapsedSeconds :type "Float (double-precision)") (TriggeredSeconds :type "Float (double-precision)") (InputAction :type "InputAction Object Reference" :default "/Game/BluePrints/Input/Action/IA_Jump.IA_Jump"))
  (bind _asbpplayer (`self.AsBpPlayer`))
  (:`Started`
    (`Character.Jump` _asbpplayer))
  (:`Completed`
    (`Character.StopJumping` _asbpplayer)))

(event `EnhancedInput|/Game/BluePrints/Input/Action/IA_Crouch`
  (params (ActionValue :type Boolean) (ElapsedSeconds :type "Float (double-precision)") (TriggeredSeconds :type "Float (double-precision)") (InputAction :type "InputAction Object Reference" :default "/Game/BluePrints/Input/Action/IA_Crouch.IA_Crouch"))
  (bind _asbpplayer (`self.AsBpPlayer`))
  (:`Started`
    (`Character.Crouch` _asbpplayer))
  (:`Completed`
    (`Character.UnCrouch` _asbpplayer)))

(event `EnhancedInput|/Game/BluePrints/Input/Action/IA_Move`
  (params (ActionValue :type "Vector2D Structure") (ElapsedSeconds :type "Float (double-precision)") (TriggeredSeconds :type "Float (double-precision)") (InputAction :type "InputAction Object Reference" :default "/Game/BluePrints/Input/Action/IA_Move.IA_Move"))
  (bind (_returnvalue_roll _returnvalue_pitch _returnvalue_yaw) (`KismetMathLibrary.BreakRotator` (`self.GetControlRotation`)))
  (bind (_returnvalue_roll_2 _returnvalue_pitch_2 _returnvalue_yaw_2) (`KismetMathLibrary.BreakRotator` (`self.GetControlRotation`)))
  (:`Triggered`
    (`Pawn.AddMovementInput` (`self.AsBpPlayer`) (`KismetMathLibrary.GetRightVector` (`KismetMathLibrary.MakeRotator` _returnvalue_roll_2 0.0 _returnvalue_yaw_2)) ActionValue_X false)
    (`Pawn.AddMovementInput` (`self.AsBpPlayer`) (`KismetMathLibrary.GetForwardVector` (`KismetMathLibrary.MakeRotator` _returnvalue_roll 0.0 _returnvalue_yaw)) ActionValue_Y false)))

(event `EnhancedInput|/Game/BluePrints/Input/Action/IA_Attack`
  (params (ActionValue :type Boolean) (ElapsedSeconds :type "Float (double-precision)") (TriggeredSeconds :type "Float (double-precision)") (InputAction :type "InputAction Object Reference" :default "/Game/BluePrints/Input/Action/IA_Attack.IA_Attack"))
  (:`Triggered`
    (`/Game/BluePrints/InGame/Charcter/Player/BP_Player.CallAttackInput` (`self.AsBpPlayer`) :!label _label))
  (:`Started`
    (goto _label)))

(fn `UserConstructionScript`)