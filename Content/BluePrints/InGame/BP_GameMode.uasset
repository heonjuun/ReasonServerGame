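; Game mode that populates the match with NPCs, runs endless rock waves and records kills and player deaths.
; On BeginPlay it spawns NPCs at random navmesh-reachable points and starts a wave of randomly counted rocks spawned high above similar points.
; A looping timer starts the next wave once no BP_Rock actors remain.
; OnHumanDeath credits the attacker's kill and flags player victims dead in their PlayerState; CheckWinner is an empty stub.
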(event `StartRockWave`
  (set `self.bRockWave` true)
  (`self.SpawnRock` (`KismetMathLibrary.RandomIntegerInRange` 5 10)))

(event `self.ReceiveBeginPlay`
  (`self.SpawnNPC` (`self.NPCSpawnCount`))
  (`self.StartRockWave`)
  (`KismetSystemLibrary.K2_SetTimerDelegate` (delegate `CheckRockWaveEnd`) 1.0 true))

(event `CheckRockWaveEnd`
  (if (`self.bRockWave`)
    (bind _outactors (`GameplayStatics.GetAllActorsOfClass` "/Game/BluePrints/InGame/Trap/BP_Rock.BP_Rock_C"))
    (if (<= (`KismetArrayLibrary.Array_Length` _outactors) 0)
      (set `self.bRockWave` false)
      (`self.StartRockWave`))))

(fn `CheckWinner`
  (if (`self.bGameIsOver`)
    _))

(fn `OnHumanDeath`
  (params (Attacker :type "/Game/BluePrints/InGame/Charcter/Player/BP_Player Object Reference") (Victim :type "/Game/BluePrints/InGame/Charcter/BP_Human Object Reference"))
  (bind _playerstate (`/Game/BluePrints/InGame/Charcter/Player/BP_Player.GetBP_PlayerState` (`local.Attacker`)))
  (`/Engine/EditorBlueprintResources/StandardMacros.IsValid` Attacker
    (:`Is Valid`
      (`/Engine/EditorBlueprintResources/StandardMacros.IsValid` Victim
        (:`Is Valid`
          (`|ExecutionSequence`
            (:`then_0`
              (`/Engine/EditorBlueprintResources/StandardMacros.IsValid` _playerstate
                (:`Is Valid`
                  (`/Engine/EditorBlueprintResources/StandardMacros.IncrementInt` (`/Game/BluePrints/InGame/Charcter/Player/BP_PlayerState.KillCount` _playerstate)))))
            (:`then_1`
              (bind _asbp_player (cast `/Game/BluePrints/InGame/Charcter/Player/BP_Player` (`local.Victim`)))
              (`self.OnPlayerDeath` (`/Game/BluePrints/InGame/Charcter/Player/BP_Player.GetBP_PlayerState` _asbp_player)))))))))

(fn `OnPlayerDeath`
  (params (PlayerState :type "/Game/BluePrints/InGame/Charcter/Player/BP_PlayerState Object Reference"))
  (set `/Game/BluePrints/InGame/Charcter/Player/BP_PlayerState.bIsDead` true PlayerState))

(fn `SpawnNPC`
  (params (Count :type Integer))
  (bind (_randomlocation _returnvalue) (`NavigationSystemV1.K2_GetRandomReachablePointInRadius` (0.0 0.0 90.0) 4000.0 null null))
  (for _ (range 1 (+ Count 1))
    (if _returnvalue
      (`|SpawnActorFromClass` "/Game/BluePrints/InGame/Charcter/NPC/BP_NPC.BP_NPC_C" (`KismetMathLibrary.MakeTransform` _randomlocation) "AdjustIfPossibleButAlwaysSpawn" "MultiplyWithRoot" null null))))

(fn `SpawnRock`
  (params (Count :type Integer))
  (if (> Count 0)
    (for _ (range 1 (+ Count 1))
      (`|SpawnActorFromClass` "/Game/BluePrints/InGame/Trap/BP_Rock.BP_Rock_C" (`KismetMathLibrary.MakeTransform` (`KismetMathLibrary.MakeVector` (.x (`NavigationSystemV1.K2_GetRandomReachablePointInRadius` (0.0 0.0 0.0) 2000.0 null null)) (.y (`NavigationSystemV1.K2_GetRandomReachablePointInRadius` (0.0 0.0 0.0) 2000.0 null null)) (+ (.z (`NavigationSystemV1.K2_GetRandomReachablePointInRadius` (0.0 0.0 0.0) 2000.0 null null)) 2000.0))) "AdjustIfPossibleButAlwaysSpawn" "MultiplyWithRoot" null null))))

(fn `UserConstructionScript`)