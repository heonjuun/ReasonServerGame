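; BP_Rock is a trap rock that damages a BP_Human it hits.
; Its static mesh hit event runs only on the authority and uses an AlreadyHit flag to resolve a single impact.
; A human hit calls ApplyRockDamage and destroys the rock.
; Hitting an actor tagged Floor stops the rock's physics and collision, then removes it after a short lifespan.
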(event `self.StaticMesh.OnComponentHit`
  (params (HitComponent :type "PrimitiveComponent Object Reference") (OtherActor :type "Actor Object Reference") (OtherComp :type "PrimitiveComponent Object Reference") (NormalImpulse :type "Vector Structure") (Hit :type "HitResult Structure (by ref)"))
  (`/Engine/EditorBlueprintResources/ActorMacros.Switch Has Authority`
    (:`Authority`
      (if (not (`self.bAlreadyHit`))
        (bind _asbp_human (cast `/Game/BluePrints/InGame/Charcter/BP_Human` OtherActor)
          (:`then`
            (set `self.bAlreadyHit` true)
            (`/Game/BluePrints/InGame/Charcter/BP_Human.ApplyRockDamage` _asbp_human (`self.Damage`))
            (`self.K2_DestroyActor`))
          (:`CastFailed`
            (if (`self.ActorHasTag` OtherActor "Floor")
              ; 바닥 충돌
              (set `self.bAlreadyHit` true)
              (`PrimitiveComponent.SetSimulatePhysics` (`self.StaticMesh`) false)
              (`PrimitiveComponent.SetCollisionEnabled` (`self.StaticMesh`) "NoCollision")
              (`self.SetLifeSpan` 1.0))))))))

(fn `UserConstructionScript`)